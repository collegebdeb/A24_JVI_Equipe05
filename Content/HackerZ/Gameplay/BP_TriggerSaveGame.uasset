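; BP_TriggerSaveGame is a one-shot checkpoint trigger that saves the game when BP_Player overlaps it.
; It passes the Capsule's world location and rotation, plus the player's current health, to HackerZGameMode's OnSave.
; The construction script divides the Capsule's relative scale and location by the Scene component's world scale, counteracting scaling applied to the actor.
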(event EventBeginPlay)

(event Collision|EventActorBeginOverlap
  (params (OtherActor :type Actor%20Object%20Reference))
  (bind _capsule (Variables|Default|GetCapsule))
  (bind _asbp_player (Utilities|Casting|CastToBP_Player OtherActor))
  (Utilities|FlowControl|DoOnce false
    (:Completed
      (bind _ashacker_zgame_mode (Utilities|Casting|CastToHackerZGameMode (Game|GetGameMode)))
      (Default|OnSave _ashacker_zgame_mode (Transformation|GetWorldLocation _capsule) (Variables|/Game/HackerZ/Blueprints/Player/BP_Player.BP_Player_C|GetHealthCurrent _asbp_player) (Transformation|GetWorldRotation _capsule)))))

(event EventTick
  (params (DeltaSeconds :type Float%20%28single-precision%29)))

(fn ConstructionScript
  (bind _capsule (Variables|Default|GetCapsule))
  (bind _capsule_2 (Variables|Default|GetCapsule))
  (Transformation|SetRelativeScale3D _capsule (/ (Variables|/Script/Engine.SceneComponent|GetRelativeScale3D _capsule) (Transformation|GetWorldScale (Variables|Default|GetScene))))
  (Transformation|SetRelativeLocation _capsule_2 (/ (Variables|/Script/Engine.SceneComponent|GetRelativeLocation _capsule_2) (Transformation|GetWorldScale (Variables|Default|GetScene))) false false))
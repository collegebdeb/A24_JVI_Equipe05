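; BP_Battery is an interactable battery that can be pulled off its parent actor once it is allowed to disconnect.
; A sphere overlap shows the WBP_Disconnect prompt to the player, while SetCanBeDisconnected turns the emissive material red or green and updates the widget through a dispatcher.
; TryDisconnectBattery, also bound to debug key B, either detaches and launches the mesh with physics and fires a detach dispatcher, or shakes the prompt through a timeline.
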(event OnComponentBeginOverlap(Sphere)
  (params (OverlappedComponent :type Primitive%20Component%20Object%20Reference) (OtherActor :type Actor%20Object%20Reference) (OtherComp :type Primitive%20Component%20Object%20Reference) (OtherBodyIndex :type Integer) (bFromSweep :type Boolean) (SweepResult :type Hit%20Result%20Structure%20%28by%20ref%29))
  (bind _widget (Variables|Default|GetWidget))
  (Utilities|Casting|CastToBP_Player OtherActor)
  (Utilities|Casting|CastToCapsuleComponent OtherComp)
  (Utilities|IsValid _widget
    (:Is%20Valid
      (Rendering|SetVisibility _widget true false)
      (if (Variables|Default|GetCanBeDisconnected)
        _))))

(event OnComponentEndOverlap(Sphere)
  (params (OverlappedComponent :type Primitive%20Component%20Object%20Reference) (OtherActor :type Actor%20Object%20Reference) (OtherComp :type Primitive%20Component%20Object%20Reference) (OtherBodyIndex :type Integer))
  (bind _widget (Variables|Default|GetWidget))
  (Utilities|Casting|CastToBP_Player OtherActor)
  (Utilities|Casting|CastToCapsuleComponent OtherComp)
  (Utilities|IsValid _widget
    (:Is%20Valid
      (Rendering|SetVisibility _widget false false))))

(event Custom|OnDisconnecedStatusChange_Event
  (Utilities|IsValid (Variables|Default|GetPromptText)
    (:Is%20Valid
      (bind _aswbp_disconnect (Utilities|Casting|CastToWBP_Disconnect (UserInterface|GetWidget (Variables|Default|GetWidget))))
      (Variables|/Game/HackerZ/HUD/WBP_Disconnect.WBP_Disconnect_C|SetCanBeDisconnected _aswbp_disconnect (Variables|Default|GetCanBeDisconnected)))))

(event Custom|ShakePrompt
  (Components|Timeline|SetPlayRate (Variables|Default|GetTimeline) 2.0)
  (bind _rotation (Timeline|Timeline PlayFromStart)
    (:Update
      (bind _aswbp_disconnect (Utilities|Casting|CastToWBP_Disconnect (UserInterface|GetWidget (Variables|Default|GetWidget))))
      (Default|Shake _aswbp_disconnect (* _rotation 15.0)))))

(event EventBeginPlay
  (bind _widget (Variables|Default|GetWidget))
  (EventDispatchers|BindEventtoOnDisconnecedStatusChange (delegate Custom|OnDisconnecedStatusChange_Event))
  (Default|CallOnDisconnecedStatusChange)
  (Utilities|IsValid _widget
    (:Is%20Valid
      (Rendering|SetVisibility _widget false false))))

(event Collision|EventActorBeginOverlap
  (params (OtherActor :type Actor%20Object%20Reference)))

(event EventTick
  (params (DeltaSeconds :type Float%20%28single-precision%29)))

(event Input|KeyboardEvents|DebugKeyB
  (params (Key :type Key%20Structure) (ActionValue :type Input%20Action%20Value%20Structure))
  (:Pressed
    (CallFunction|TryDisconnectBattery)))

(fn ConstructionScript
  (bind _returnvalue (Rendering|Material|CreateDynamicMaterialInstance (Variables|Default|GetStaticMesh) 1 "/Game/HackerZ/Materials/MI_Battery_Emissive.MI_Battery_Emissive" "None" :!class /Script/Engine.PrimitiveComponent))
  (bind _output_get (Variables|Default|SetEmissiveMatRef _returnvalue))
  (Rendering|Material|SetVectorParameterValue _output_get "EmissiveColor" "(R=1.000000,G=0.000000,B=0.000000,A=1.000000)" :!class /Script/Engine.MaterialInstanceDynamic))

(fn TryDisconnectBattery
  (bind _staticmesh (Variables|Default|GetStaticMesh))
  (if (Variables|Default|GetCanBeDisconnected)
    (Development|PrintString (Utilities|String|Append "Retire la batterie de : " (Utilities|GetDisplayName (Actor|GetAttachParentActor))))
    (Transformation|DetachFromActor "KeepWorld" "KeepWorld" "KeepWorld")
    (Physics|SetSimulatePhysics (Variables|Default|GetStaticMesh) true)
    (Physics|SetPhysicsLinearVelocity _staticmesh "0, 0, 0" false "None")
    (Physics|AddImpulse _staticmesh (+ (* (Math|Vector|GetUpVector _staticmesh) 1e+02) "0.000000,0.000000,200.000000") "None" true)
    (Components|DestroyComponent (Variables|Default|GetCantPromptText))
    (Default|CallOnDetach)
    (else
      (CallFunction|ShakePrompt))))

(fn SetCanbeDisconnected
  (params (CanBeDisconnected :type Boolean))
  (bind _emissivematref (Variables|Default|GetEmissiveMatRef))
  (bind _output_get (Variables|Default|SetCanBeDisconnected CanBeDisconnected))
  (Default|CallOnDisconnecedStatusChange)
  (if _output_get
    (Rendering|Material|SetVectorParameterValue _emissivematref "EmissiveColor" "(R=0.140267,G=1.000000,B=0.000000,A=1.000000)" :!class /Script/Engine.MaterialInstanceDynamic)
    (else
      (Rendering|Material|SetVectorParameterValue _emissivematref "EmissiveColor" "(R=1.000000,G=0.000000,B=0.000000,A=1.000000)" :!class /Script/Engine.MaterialInstanceDynamic))))
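; BP_Transporter is a portal that teleports BP_Player to its EndPoint, with a looping timeline animating the sphere's scale.
; Trigger overlap disables input, shakes the camera and plays a timeline driving camera post-process and Scene scale to mask the jump.
; After teleporting, a second timeline restores the saved post-process and input while animating Scene scale.
; The construction script applies the portal color to materials, Niagara particles and spotlight, and emissive intensity to materials and particles.
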(event OnComponentBeginOverlap(Trigger)
  (params (OverlappedComponent :type Primitive%20Component%20Object%20Reference) (OtherActor :type Actor%20Object%20Reference) (OtherComp :type Primitive%20Component%20Object%20Reference) (OtherBodyIndex :type Integer) (bFromSweep :type Boolean) (SweepResult :type Hit%20Result%20Structure%20%28by%20ref%29))
  (bind _asbp_player (Utilities|Casting|CastToBP_Player OtherActor))
  (Input|DisableInput _asbp_player 0)
  (Camera|PlayWorldCameraShake "/Game/HackerZ/Blueprints/Player/FirstPerson/PlayerCameraShake.PlayerCameraShake_C" (Transformation|GetWorldLocation (Variables|/Game/HackerZ/Blueprints/Player/BP_Player.BP_Player_C|GetFirstPersonCamera _asbp_player)) 0.0 5e+02)
  (bind _output_get (Variables|Default|SetOriginalValues (Variables|/Script/Engine.CameraComponent|GetPostProcessSettings (Variables|/Game/HackerZ/Blueprints/Player/BP_Player.BP_Player_C|GetFirstPersonCamera _asbp_player))))
  (bind _gain (Timeline|ColorgradeEnd Play)
    (:Update
      (Variables|/Script/Engine.CameraComponent|SetPostProcessSettings (Variables|/Game/HackerZ/Blueprints/Player/BP_Player.BP_Player_C|GetFirstPersonCamera _asbp_player) (Utilities|Struct|MakePostProcessSettings (+ (* _gain 1e+01) 11.0)))
      (Transformation|SetRelativeScale3D (Variables|Default|GetScene) (Math|Conversions|ToVector(Float) (+ (* _gain 2.5) 1.0))))
    (:Finished
      (bind _returnvalue (Actor|GetActorOfClass "/Game/HackerZ/Blueprints/Player/BP_Player.BP_Player_C"))
      (Transformation|SetActorTransform _returnvalue (Transformation|GetActorTransform (Variables|Default|GetEndPoint)))
      (bind _gain_2 (Timeline|Timeline Play)
        (:Update
          (Variables|/Script/Engine.CameraComponent|SetPostProcessSettings (Variables|/Game/HackerZ/Blueprints/Player/BP_Player.BP_Player_C|GetFirstPersonCamera _asbp_player) _output_get)
          (Transformation|SetRelativeScale3D (Variables|Default|GetScene) (Math|Conversions|ToVector(Float) (+ (* _gain_2 2.5) 1.0)))
          (Input|EnableInput _asbp_player 0))))))

(event EventBeginPlay
  (Components|Timeline|SetLooping (Variables|Default|GetPortalTimeline) true)
  (bind _scale (Timeline|PortalTimeline Play)
    (:Update
      (Transformation|SetRelativeScale3D (Variables|Default|GetSphere) (Math|Conversions|ToVector(Float) _scale)))))

(event Collision|EventActorBeginOverlap
  (params (OtherActor :type Actor%20Object%20Reference)))

(event EventTick
  (params (DeltaSeconds :type Float%20%28single-precision%29)))

(fn ConstructionScript
  (Rendering|Material|SetVectorParameterValueonMaterials (Variables|Default|GetRing) "EmissiveColor" (Math|Conversions|ToVector(LinearColor) (Variables|Default|GetPortalColor)))
  (Rendering|Material|SetScalarParameterValueonMaterials (Variables|Default|GetRing) "EmissiveIntensity" (Variables|Default|GetEmissiveIntensity))
  (Effects|Components|ParticleSystem|SetColorParameter (Variables|Default|GetNiagara) "User.ParticleColor" (* (Variables|Default|GetPortalColor) (Variables|Default|GetEmissiveIntensity)))
  (Rendering|Components|Light|SetLightColor (Variables|Default|GetSpotLight) (Variables|Default|GetPortalColor) true)
  (Variables|Default|SetSphereScale (.x (Variables|/Script/Engine.SceneComponent|GetRelativeScale3D (Variables|Default|GetSphere)))))